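; Enemy pawn that chases the player once its PawnSensing component spots a pawn.
; Seeing a pawn sets IsSeeingPlayer, which is never cleared here, and calls FollowPlayer to issue an AI MoveTo toward player 0.
; FollowPlayer calls itself straight from the move node's immediate output, without waiting for success or failure.
; Random-point roaming is unfinished: its move-and-delay loop is disconnected, leaving Roam empty.
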(event OnSeePawn(PawnSensing)
  (params (Pawn :type Pawn%20Object%20Reference))
  ;[1 1 1] See Pawn
  (Variables|Default|SetIsSeeingPlayer? true)
  (CallFunction|FollowPlayer))

(event Custom|FollowPlayer
  ;[1 1 1] Follow Player Event
  (if (Variables|Default|GetIsSeeingPlayer?)
    (AI|AIMoveTo self "0, 0, 0" (Game|GetPlayerCharacter 0) 5.0 false
      (:then
        (CallFunction|FollowPlayer)))))

(event Custom|Roam)

(event EventBeginPlay)

(event Collision|EventActorBeginOverlap
  (params (OtherActor :type Actor%20Object%20Reference)))

(event EventTick
  (params (DeltaSeconds :type Float%20%28single-precision%29)))

(fn ConstructionScript)