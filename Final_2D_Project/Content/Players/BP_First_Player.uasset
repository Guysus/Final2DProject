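; Player character for a 2D side-view brawler: Enhanced Input drives walking, punching and kicking by swapping sprite flipbooks, with vertical position clamped to a band.
; BeginPlay detaches the camera, fills health and updates the controller's health bar.
; Tick snaps camera X to the player past a screen-space threshold.
; It also opens the pause menu (the close branch is unreachable) and shows a death menu at zero health.
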(event Custom|Player%20Dead
  ;[1 1 1] Player Dead
  (if (== (Variables|Default|GetCurrentHealth) 0.0)
    (Actor|DestroyActor)
    (bind _returnvalue (UserInterface|CreateWidget "/Game/Widgets/WB_Death_Menu.WB_Death_Menu_C"))
    (UserInterface|Viewport|AddtoViewport _returnvalue 0)))

(event Input|EnhancedActionEvents|EnhancedInputActionIA_Walk_Left_Right
  (params (ActionValue :type Float%20%28double-precision%29) (ElapsedSeconds :type Float%20%28double-precision%29) (TriggeredSeconds :type Float%20%28double-precision%29) (InputAction :type Input%20Action%20Object%20Reference :default "/Game/Blueprints/IA_Walk_Left_Right.IA_Walk_Left_Right"))
  (bind _returnvalue (Transformation|GetActorLocation))
  ;[1 1 1] Player Movement Left/Right
  (:Triggered
    (Pawn|Input|AddMovementInput "1.000000,0.000000,0.000000" ActionValue false)
    (Transformation|SetActorLocation (Math|Vector|MakeVector (.x _returnvalue) (.y _returnvalue) (Math|Float|Clamp(Float) (.z _returnvalue) 123.0 345.0)) false false)
    (if (> ActionValue 0.0)
      (Transformation|SetWorldRotation (Variables|Default|GetSprite) "0, 0, 0" false false)
      (Sprite|SetFlipbook (Variables|Default|GetSprite) "/Game/Sprites/A_Walk.A_Walk")
      (elif (< ActionValue 0.0)
        (Transformation|SetWorldRotation (Variables|Default|GetSprite) "0.000000,180.000000,0.000000" false false)
        (Sprite|SetFlipbook (Variables|Default|GetSprite) "/Game/Sprites/A_Walk.A_Walk"))))
  (:Completed
    (Sprite|SetFlipbook (Variables|Default|GetSprite) "/Game/Sprites/A_Idle.A_Idle")))

(event Input|EnhancedActionEvents|EnhancedInputActionIA_Walk_Up_Down
  (params (ActionValue :type Float%20%28double-precision%29) (ElapsedSeconds :type Float%20%28double-precision%29) (TriggeredSeconds :type Float%20%28double-precision%29) (InputAction :type Input%20Action%20Object%20Reference :default "/Game/Blueprints/IA_Walk_Up_Down.IA_Walk_Up_Down"))
  (bind _returnvalue (Transformation|GetActorLocation))
  (:Triggered
    (Pawn|Input|AddMovementInput "0.000000,0.000000,-1.000000" ActionValue false)
    (Transformation|SetActorLocation (Math|Vector|MakeVector (.x _returnvalue) (.y _returnvalue) (Math|Float|Clamp(Float) (.z _returnvalue) 123.0 345.0)) false false)
    (if (> ActionValue 0.0)
      (Transformation|SetWorldRotation (Variables|Default|GetSprite) "0, 0, 0" false false)
      (Sprite|SetFlipbook (Variables|Default|GetSprite) "/Game/Sprites/A_Walk.A_Walk")
      (elif (< ActionValue 0.0)
        (Transformation|SetWorldRotation (Variables|Default|GetSprite) "0, 0, 0" false false)
        (Sprite|SetFlipbook (Variables|Default|GetSprite) "/Game/Sprites/A_Walk.A_Walk"))))
  (:Completed
    (Sprite|SetFlipbook (Variables|Default|GetSprite) "/Game/Sprites/A_Idle.A_Idle")))

(event Input|EnhancedActionEvents|EnhancedInputActionIA_Punch
  (params (ActionValue :type Boolean) (ElapsedSeconds :type Float%20%28double-precision%29) (TriggeredSeconds :type Float%20%28double-precision%29) (InputAction :type Input%20Action%20Object%20Reference :default "/Game/Blueprints/IA_Punch.IA_Punch"))
  (:Triggered
    (Sprite|SetFlipbook (Variables|Default|GetSprite) "/Game/Sprites/A_Punch.A_Punch"))
  (:Completed
    (Sprite|SetFlipbook (Variables|Default|GetSprite) "/Game/Sprites/A_Idle.A_Idle")))

(event Input|EnhancedActionEvents|EnhancedInputActionIA_Kick
  (params (ActionValue :type Boolean) (ElapsedSeconds :type Float%20%28double-precision%29) (TriggeredSeconds :type Float%20%28double-precision%29) (InputAction :type Input%20Action%20Object%20Reference :default "/Game/Blueprints/IA_Kick.IA_Kick"))
  (:Triggered
    (Sprite|SetFlipbook (Variables|Default|GetSprite) "/Game/Sprites/A_Kick.A_Kick"))
  (:Completed
    (Sprite|SetFlipbook (Variables|Default|GetSprite) "/Game/Sprites/A_Idle.A_Idle")))

(event Input|EnhancedActionEvents|EnhancedInputActionIA_Pause_Game
  (params (ActionValue :type Boolean) (ElapsedSeconds :type Float%20%28double-precision%29) (TriggeredSeconds :type Float%20%28double-precision%29) (InputAction :type Input%20Action%20Object%20Reference :default "/Game/Blueprints/IA_Pause_Game.IA_Pause_Game"))
  (bind _returnvalue (Game|GetPlayerController 0))
  ;[1 1 1] Pause Menu
  (:Started
    (if true
      (Variables|Default|SetIsPauseMenuOpened? true)
      (bind _returnvalue_2 (UserInterface|CreateWidget "/Game/Widgets/WB_Pause_Menu.WB_Pause_Menu_C" _returnvalue))
      (bind _output_get (Variables|Default|SetPause%20Menu%20Widget _returnvalue_2))
      (UserInterface|Viewport|AddtoViewport _output_get 0)
      (Input|SetInputModeGameandUI _returnvalue (Variables|Default|GetPause%20Menu%20Widget) "DoNotLock" true false)
      (Variables|/Script/Engine.PlayerController|SetbShowMouseCursor (Game|GetPlayerController 0) true)
      (Game|SetGamePaused true)
      (else
        (Variables|Default|SetIsPauseMenuOpened? false)
        (Widget|RemovefromParent (Variables|Default|GetPause%20Menu%20Widget))
        (Game|SetGamePaused false)
        (Input|SetInputModeGameOnly _returnvalue false)
        (Variables|/Script/Engine.PlayerController|SetbShowMouseCursor (Game|GetPlayerController 0) false)))))

(event EventBeginPlay
  ;[1 1 1] Begin Play
  (Transformation|DetachFromComponent (Variables|Default|GetCamera) "KeepWorld" "KeepWorld" "KeepWorld" true)
  (Variables|Default|SetCurrentHealth (Variables|Default|GetMaxHealth))
  (bind _asbp_first_controller (Utilities|Casting|CastToBP_First_Controller (Pawn|GetController)))
  (Default|UpdateHealthBar _asbp_first_controller (Variables|Default|GetCurrentHealth) (Variables|Default|GetMaxHealth))
  (Input|AddMappingContext (PlayerController|LocalPlayerSubsystems|GetEnhancedInputLocalPlayerSubsystem _asbp_first_controller) "/Game/Blueprints/InputMappingContext.InputMappingContext" 0 "(bIgnoreAllPressedKeysUntilRelease=True,bForceImmediately=False,bNotifyUserSettings=False)"))

(event Collision|EventActorBeginOverlap
  (params (OtherActor :type Actor%20Object%20Reference)))

(event EventTick
  (params (DeltaSeconds :type Float%20%28single-precision%29))
  (bind _camera (Variables|Default|GetCamera))
  (bind _returnvalue (Transformation|GetWorldLocation _camera))
  ;[1 1 1] Event Tick
  (Development|PrintString "Hello" true true "(R=0.000000,G=0.660000,B=1.000000,A=1.000000)" 1e-05)
  (if (> (.x (.ScreenLocation (Class|PlayerController|ProjectWorldLocationtoScreen (Game|GetPlayerController 0) (Transformation|GetActorLocation) false))) 2.1e+03)
    (Transformation|SetWorldLocation _camera (Math|Vector|MakeVector (.x (Transformation|GetActorLocation)) (.y _returnvalue) (.z _returnvalue)) false false)))

(fn ConstructionScript)